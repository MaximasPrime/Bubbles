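; Player drink cup that visually updates its liquid material as ingredients are added.
; On BeginPlay it creates a dynamic material and binds to the GI_Bubbles IngredientAdded event.
; Each event looks up the ingredient's colour in the alcohol, fruit or mixer DataTable by 1-based index.
; A timeline then animates scalar "P" through that type's range and blends the colour, with fruit resetting the base colour first.
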(event Custom|Ingredient%20Added_Event
  (params (Type :type E_IngredientType%20Enum :default "NewEnumerator0") (Index :type Integer))
  (bind _returnvalue (Utilities|Select :Index Type :NewEnumerator0 "/Game/Core/DT_Alcohol.DT_Alcohol" :NewEnumerator1 "/Game/Core/DT_Fruit.DT_Fruit" :NewEnumerator2 "/Game/Core/DT_Mixer.DT_Mixer"))
  (bind _dynamic_material (Variables|Default|GetDynamic%20Material))
  (Utilities|FlowControl|Sequence
    (:then_0
      (bind _outrownames (DataTable|GetDataTableRowNames _returnvalue))
      (bind _returnvalue_2 (Utilities|GetDataTableRow _returnvalue (Utilities|Array|Get(acopy) _outrownames (- Index 1)))
        (:then
          (Variables|Default|SetNext%20Col (.Colour (Utilities|Struct|BreakST_Ingredient _returnvalue_2))))))
    (:then_1
      (if (Utilities|Enum|Equal(Enum) Type "NewEnumerator1")
        (Variables|Default|SetColour (Variables|Default|GetNext%20Col))))
    (:then_2
      (bind _newtrack_0 (Timeline|Timeline PlayFromStart)
        (:Update
          (Rendering|Material|SetScalarParameterValue _dynamic_material "P" (Math|Float|Lerp (Utilities|Select :Index Type :NewEnumerator0 0.1 :NewEnumerator1 0.0 :NewEnumerator2 0.5) (Utilities|Select :Index Type :NewEnumerator0 0.5 :NewEnumerator1 0.1 :NewEnumerator2 1.0) _newtrack_0) :!class /Script/Engine.MaterialInstanceDynamic)
          (Rendering|Material|SetVectorParameterValue _dynamic_material "Colour" (Utilities|Struct|MakeLinearColor (.R (Math|Color|BreakColor (Math|Color|Lerp(LinearColor) (Variables|Default|GetColour) (+ (/ (Variables|Default|GetColour) 1e+01) (/ (Variables|Default|GetNext%20Col) 1e+01)) _newtrack_0))) (.G (Math|Color|BreakColor (Math|Color|Lerp(LinearColor) (Variables|Default|GetColour) (+ (/ (Variables|Default|GetColour) 1e+01) (/ (Variables|Default|GetNext%20Col) 1e+01)) _newtrack_0))) (.B (Math|Color|BreakColor (Math|Color|Lerp(LinearColor) (Variables|Default|GetColour) (+ (/ (Variables|Default|GetColour) 1e+01) (/ (Variables|Default|GetNext%20Col) 1e+01)) _newtrack_0))) 1.0) :!class /Script/Engine.MaterialInstanceDynamic))
        (:Finished
          (Variables|Default|SetColour (Utilities|Struct|MakeLinearColor (.R (Math|Color|BreakColor (Math|Color|Lerp(LinearColor) (Variables|Default|GetColour) (+ (/ (Variables|Default|GetColour) 1e+01) (/ (Variables|Default|GetNext%20Col) 1e+01)) _newtrack_0))) (.G (Math|Color|BreakColor (Math|Color|Lerp(LinearColor) (Variables|Default|GetColour) (+ (/ (Variables|Default|GetColour) 1e+01) (/ (Variables|Default|GetNext%20Col) 1e+01)) _newtrack_0))) (.B (Math|Color|BreakColor (Math|Color|Lerp(LinearColor) (Variables|Default|GetColour) (+ (/ (Variables|Default|GetColour) 1e+01) (/ (Variables|Default|GetNext%20Col) 1e+01)) _newtrack_0))) 1.0)))))))

(event EventBeginPlay
  (bind _returnvalue (Rendering|Material|CreateDynamicMaterialInstance (Variables|Default|GetStaticMesh) 1 "/Game/UI/M_Drink_Inst.M_Drink_Inst" "None" :!class /Script/Engine.PrimitiveComponent))
  (Variables|Default|SetDynamic%20Material _returnvalue)
  (bind _asgi_bubbles (Utilities|Casting|CastToGI_Bubbles (Game|GetGameInstance)))
  (bind _output_get (Variables|Default|Set%20Bubbles%20Instance _asgi_bubbles))
  (EventDispatchers|AssignIngredientAdded _output_get (delegate Custom|Ingredient%20Added_Event)))

(event Collision|EventActorBeginOverlap
  (params (OtherActor :type Actor%20Object%20Reference)))

(event EventTick
  (params (DeltaSeconds :type Float%20%28single-precision%29)))

(fn ConstructionScript)